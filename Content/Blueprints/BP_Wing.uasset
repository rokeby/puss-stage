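; BP_Wing is a wing actor whose mesh appearance is configured through variables.
; Its Construction Script passes them to ApplyWingAppearance, which sets the Cube component's mesh, relative transform and visibility only when UseAssignedMesh is true.
; A near-zero scale falls back to unit scale.
; The event graph has no active logic, and SetLateralAlpha is an empty event.
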(event `SetLateralAlpha`
  (params (alpha :type "AlphaBlend Structure")))

(fn `ApplyWingAppearance`
  (params (UseNewMesh :type Boolean) (NewMesh :type "StaticMesh Object Reference") (NewOffset :type "Vector Structure") (NewRotation :type "Rotator Structure") (NewScale :type "Vector Structure") (NewVisible :type Boolean))
  (bind _cube (`self.Cube`))
  (if UseNewMesh
    (`StaticMeshComponent.SetStaticMesh` _cube NewMesh)
    (`SceneComponent.K2_SetRelativeLocationAndRotation` _cube NewOffset NewRotation false true)
    (`SceneComponent.SetRelativeScale3D` _cube (select `bool` (`KismetMathLibrary.Vector_IsNearlyZero` NewScale) :`false` NewScale :`true` (`KismetMathLibrary.MakeVector` 1.0 1.0 1.0)))
    (`SceneComponent.SetVisibility` _cube NewVisible true)))

(fn `UserConstructionScript`
  (`self.ApplyWingAppearance` (`self.UseAssignedMesh`) (`self.AssignedMesh`) (`self.MeshOffset`) (`self.MeshRotation`) (`self.MeshScale`) (`self.WingVisible`)))